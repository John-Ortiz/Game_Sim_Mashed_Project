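; Enemy character Blueprint that chases the player and plays an attack montage after spotting a pawn.
; PawnSensing sets PlayerSeen and calls FollowPlayer, which issues AIMoveTo toward player 0; until a pawn is seen, Tick halts movement.
; The move node's then output plays the Test montage, with CanAttack restored after a montage-length delay, though each FollowPlayer call also resets it.
; PlayerSeen effectively never clears once set.
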(event OnSeePawn(PawnSensing)
  (params (Pawn :type Pawn%20Object%20Reference))
  (Variables|Default|SetPlayerSeen true)
  (CallFunction|FollowPlayer))

(event Custom|FollowPlayer
  (Variables|Default|SetCanAttack true)
  (if (Variables|Default|GetPlayerSeen)
    (AI|AIMoveTo self "0, 0, 0" (Game|GetPlayerCharacter 0) 5.0 false
      (:then
        (if (Variables|Default|GetCanAttack)
          (Variables|Default|SetCanAttack false)
          (bind _returnvalue (Animation|PlayAnimMontage "/Game/Characters/Mannequins/Animations/Manny/test.test" 1.0 "None"))
          (Utilities|FlowControl|Delay _returnvalue)
          (Variables|Default|SetCanAttack true))))
    (else
      (Variables|Default|SetPlayerSeen false))))

(event EventBeginPlay)

(event Collision|EventActorBeginOverlap
  (params (OtherActor :type Actor%20Object%20Reference)))

(event EventTick
  (params (DeltaSeconds :type Float%20%28single-precision%29))
  (if (not (Variables|Default|GetPlayerSeen))
    (Components|Movement|StopMovementImmediately (Variables|Character|GetCharacterMovement))))

(fn ConstructionScript)